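; BP_Button is an interactable button that starts spawning on a referenced Spawner when pressed.
; On BeginPlay it gets the W_Interact from its InteractionWidget, passes it a self reference and the button name as title, and binds to its press dispatcher.
; The press event calls FPushButton, which calls StartSpawn on the Spawner or prints a warning if that reference is invalid.
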(event Custom|Disp_ButtonPressed_Event
  (CallFunction|FPushButton) ; Interaction
)

(event EventBeginPlay
  (bind _asw_interact (Utilities|Casting|CastToW_Interact (UserInterface|GetUserWidgetObject (Variables|Default|GetInteractionWidget))))
  (EventDispatchers|AssignDispButtonPressed _asw_interact (delegate Custom|Disp_ButtonPressed_Event))
  (Variables|/Game/UI/W_Interact.W_Interact_C|SetBP_ButtonRef _asw_interact self)
  (Variables|/Game/UI/W_Interact.W_Interact_C|SetTitleText _asw_interact (Variables|Button|GetButtonName)) ; Set name in Widget
)

(fn ConstructionScript)

(fn FPushButton
  (bind _spawner (Variables|Button|GetSpawner)
    (:then
      (Class|TurtleSpawner|StartSpawn _spawner))
    (:else
      (Development|PrintString "No Spawner Reference"))))